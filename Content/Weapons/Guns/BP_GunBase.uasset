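; BP_GunBase is a gun Blueprint, named as a base class, that fires projectiles in single-shot or automatic mode.
; StartFire fires at once and, if CanAuto is set, starts a looping timer that repeats Fire at the FireRate interval until StopFire clears it.
; Each Fire spawns a BP_ProjectileBase at the world transform of the skeletal mesh's MuzzleSocket.
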(event `StartFire`
  (`self.Fire`)
  (if (`self.CanAuto`)
    (`KismetSystemLibrary.K2_ClearAndInvalidateTimerHandle` (`self.FireTimer`))
    (bind _returnvalue (`KismetSystemLibrary.K2_SetTimerDelegate` (delegate `Fire`) (`self.FireRate`) true))
    (set `self.FireTimer` _returnvalue)))

(event `Fire`
  (`|SpawnActorFromClass` "/Game/Weapons/Guns/BP_ProjectileBase.BP_ProjectileBase_C" (`SceneComponent.GetSocketTransform` (`self.SkeletalMesh`) "MuzzleSocket" "RTS_World") "Undefined" "OverrideRootScale" null null))

(event `StopFire`
  (`KismetSystemLibrary.K2_ClearAndInvalidateTimerHandle` (`self.FireTimer`)))

(fn `UserConstructionScript`)