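; BP_GI is a Game Instance Blueprint that manages the game's save data across the session.
; On Init it loads the BP_SaveGame from the configured slot, creating a fresh object if the slot is empty or the cast fails, and caches it in SaveGameRef.
; On Shutdown it writes that cached object back to the same slot if it is valid, without handling a failed save.
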(event `self.ReceiveInit`
  (`self.LoadSaveGame`))

(event `self.ReceiveShutdown`
  (`self.MaybeWriteSaveGame`))

(fn `LoadSaveGame`
  (bind _returnvalue (`GameplayStatics.DoesSaveGameExist` (`self.SaveGameSlotName`)))
  (if _returnvalue
    (bind _returnvalue_2 (`GameplayStatics.LoadGameFromSlot` (`self.SaveGameSlotName`)))
    (bind _asbp_save_game (cast `/Game/Blueprints/BP_SaveGame` _returnvalue_2)
      (:`then`
        (set `self.SaveGameRef` _asbp_save_game))
      (:`CastFailed`
        (bind _returnvalue_3 (`GameplayStatics.CreateSaveGameObject` "/Game/Blueprints/BP_SaveGame.BP_SaveGame_C" :!label _label))
        (set `self.SaveGameRef` _returnvalue_3)))
    (else
      (goto _label))))

(fn `MaybeWriteSaveGame`
  (`/Engine/EditorBlueprintResources/StandardMacros.IsValid` (`self.SaveGameRef`)
    (:`Is Valid`
      (bind _returnvalue (`GameplayStatics.SaveGameToSlot` (`self.SaveGameRef`) (`self.SaveGameSlotName`)))
      (if _returnvalue
        _))))