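; BP_FruitItem is a fruit item actor that supplies a camera transform for framing its static mesh.
; GetFitCameraTransform places the view at a small fixed diagonal world-space offset from the mesh's location, plus its unit forward vector, and rotates it to look at the mesh.
; The offset ignores mesh bounds, and the event graph and construction script add no behavior of their own.
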(fn `GetFitCameraTransform`
  (returns (Ret :type "Transform Structure"))
  (bind _staticmesh (`self.StaticMesh`))
  (bind _returnvalue (`SceneComponent.K2_GetComponentLocation` _staticmesh))
  (bind _returnvalue_2 (+ _returnvalue (+ (* (`SceneComponent.GetForwardVector` _staticmesh) 1.0) (20.0 20.0 20.0))))
  (return (`KismetMathLibrary.MakeTransform` _returnvalue_2 (`KismetMathLibrary.FindLookAtRotation` _returnvalue_2 _returnvalue))))

(fn `UserConstructionScript`
  (`parent.UserConstructionScript`))