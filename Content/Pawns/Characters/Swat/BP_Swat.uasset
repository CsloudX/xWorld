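; BP_Swat is a SWAT character pawn that carries an AK and can be killed by damage.
; On BeginPlay it spawns a BP_AK, stores it as the equipped weapon and snaps it to the mesh's RightHandSocket.
; AnyDamage subtracts from Health and, at zero or below, turns on mesh collision and physics simulation so the body ragdolls.
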(event `self.ReceiveBeginPlay`
  (bind _returnvalue (`|SpawnActorFromClass` "/Game/Weapons/Guns/AK/BP_AK.BP_AK_C" (`KismetMathLibrary.MakeTransform` (0.0 0.0 0.0)) "Undefined" "OverrideRootScale" null null))
  (bind _output_get (set `self.EquippedWeapon` _returnvalue))
  (`self.K2_AttachToComponent` _output_get (`self.Mesh`) "RightHandSocket" "SnapToTarget" "SnapToTarget" "SnapToTarget" true))

(event `self.ReceiveAnyDamage`
  (params (Damage :type "Float (single-precision)") (DamageType :type "DamageType Object Reference") (InstigatedBy :type "Controller Object Reference") (DamageCauser :type "Actor Object Reference"))
  (bind _mesh (`self.Mesh`))
  (bind _output_get (set `self.Health` (- (`self.Health`) Damage)))
  (if (<= _output_get 0.0)
    (`PrimitiveComponent.SetCollisionEnabled` _mesh "QueryAndPhysics")
    (`PrimitiveComponent.SetSimulatePhysics` _mesh true)))

(fn `UserConstructionScript`
  (`parent.UserConstructionScript`))