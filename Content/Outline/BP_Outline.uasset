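; BP_Outline is an actor that displays a configurable static mesh and can toggle a colored outline on it.
; CreateOutline spawns an unattached duplicate mesh component at the mesh's world transform, with a dynamic M_Outline material on slot 0 fed by Color and Scale.
; DeleteOutline destroys that component, while the HasOutline flag prevents duplicates.
; The construction script applies the chosen Mesh, and both events print debug messages.
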(event `self.ReceiveBeginPlay`)

(event `CreateOutline`
  (`KismetSystemLibrary.PrintString` "Create Outline")
  (if (not (`self.HasOutline`))
    (bind _returnvalue (`AddComponent|NODE_AddStaticMeshComponent-0` :`bManualAttachment` true :`RelativeTransform` (`SceneComponent.K2_GetComponentToWorld` (`self.StaticMesh`))))
    (bind _output_get (set `self.MeshComponent` _returnvalue))
    (`StaticMeshComponent.SetStaticMesh` _output_get (`self.Mesh`))
    (bind _returnvalue_2 (`PrimitiveComponent.CreateDynamicMaterialInstance` _output_get 0 "/Game/Outline/M_Outline.M_Outline" "None"))
    (`MaterialInstanceDynamic.SetVectorParameterValue` _returnvalue_2 "Color" (`self.Color`))
    (`MaterialInstanceDynamic.SetScalarParameterValue` _returnvalue_2 "Scale" (`self.Scale`))
    (set `self.HasOutline` true)))

(event `DeleteOutline`
  (bind _meshcomponent (`self.MeshComponent`))
  (`KismetSystemLibrary.PrintString` "Delete Outline")
  (`/Engine/EditorBlueprintResources/StandardMacros.IsValid` _meshcomponent
    (:`Is Valid`
      (`ActorComponent.K2_DestroyComponent` _meshcomponent)
      (set `self.HasOutline` false))))

(fn `UserConstructionScript`
  (`StaticMeshComponent.SetStaticMesh` (`self.StaticMesh`) (`self.Mesh`)))