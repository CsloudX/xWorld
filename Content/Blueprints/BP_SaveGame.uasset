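; BP_SaveGame is a save game Blueprint that holds the player's info and exposes a getter and setter for it.
; SetPlayerInfo compares only the Name field, and on a difference it stores the new struct, flags IsNeedSave and broadcasts PlayerInfoChanged.
; The file only marks the data as needing a save and does not write it to a slot itself.
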(fn `GetPlayerInfo`
  (returns (PlayerInfo :type "/Game/Structures/S_PlayerInfo Structure"))
  (return (`self.PlayerInfo`)))

(fn `SetPlayerInfo`
  (params (PlayerInfo :type "/Game/Structures/S_PlayerInfo Structure"))
  (if (`KismetTextLibrary.NotEqual_TextText` (`.Name_3_AF95FE6549D18BECC4A13BA09865E2AD` (break `/Game/Structures/S_PlayerInfo` PlayerInfo)) (`.Name_3_AF95FE6549D18BECC4A13BA09865E2AD` (break `/Game/Structures/S_PlayerInfo` (`self.PlayerInfo`))))
    (set `self.PlayerInfo` PlayerInfo)
    (set `self.IsNeedSave` true)
    (`self.PlayerInfoChanged` (`self.PlayerInfo`))))